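; BP_Stage is a stage actor made of base and border meshes that can spawn strawberries.
; On BeginPlay it turns both meshes black when the current level is L_One_Dark.
; The SpawningStrawberry event spawns a BP_Strawberry at the StrawberryPosition component's location with a fixed tilt.
; A random red, blue, yellow or green recolor of both meshes is left unconnected and never runs.
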(event Custom|SpawningStrawberry
  (Game|SpawnActorfromClass "/Game/Blueprints/Actors/BP_Strawberry.BP_Strawberry_C" (Math|Transform|MakeTransform (Transformation|GetWorldLocation (Variables|Default|GetStrawberryPosition)) "0.000000,0.000000,20.000000" "1.000000,1.000000,1.000000") "Undefined" "MultiplyWithRoot" 0 0))

(event EventBeginPlay
  (bind _returnvalue (Game|GetCurrentLevelName true))
  (if (not (not (Utilities|Enum|Equal(Enum) _returnvalue "L_One_Dark")))
    (Rendering|Material|SetMaterial (Variables|Default|GetStageBase) 0 "/Game/Materials/M_Black.M_Black")
    (Rendering|Material|SetMaterial (Variables|Default|GetStageBorders) 0 "/Game/Materials/M_Black.M_Black")))

(fn ConstructionScript)