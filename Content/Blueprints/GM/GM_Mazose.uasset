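; GM_Mazose is a game mode that handles level audio, the start countdown and respawn-platform removal for a ball game.
; On BeginPlay it binds play and stop events for its audio and, on levels prefixed "L_", adds the WB_CountHUD countdown widget to the viewport.
; Its RespawnElimination event destroys the BP_RespawnPlatform when exactly one exists, then has BP_BallPlayerController put up the level HUD.
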(event Custom|PlayingSound
  (Audio|Components|Audio|Play (Variables|Default|GetAudio) 0.0))

(event Custom|QuittingSound
  (Audio|Components|Audio|Stop (Variables|Default|GetAudio)))

(event Custom|CountdownSet
  (bind _returnvalue (UserInterface|CreateWidget "/Game/Blueprints/Widgets/WB_CountHUD.WB_CountHUD_C" (Game|GetPlayerController 0)))
  (UserInterface|Viewport|AddtoViewport _returnvalue 0))

(event Custom|RespawnElimination
  (CallFunction|DestroyingRespawnPlatform)
  (CallFunction|StartingLevelHUD))

(event EventBeginPlay
  (Utilities|FlowControl|Sequence
    (:then_0
      (EventDispatchers|BindEventtoPlaySound (delegate Custom|PlayingSound))
      (EventDispatchers|BindEventtoStopSound (delegate Custom|QuittingSound)))
    (:then_1
      (CallFunction|SettingCountdownonPlayableLevels))))

(fn ConstructionScript)

(fn SettingCountdownonPlayableLevels
  (bind _returnvalue (Game|GetCurrentLevelName true))
  (if (Utilities|String|StartsWith _returnvalue "L_")
    (CallFunction|CountdownSet)))

(fn DestroyingRespawnPlatform
  (bind _outactors (Actor|GetAllActorsOfClass "/Game/Blueprints/Actors/BP_RespawnPlatform.BP_RespawnPlatform_C"))
  (if (== (Utilities|Array|Length _outactors) 1)
    (Utilities|IsValid (Utilities|Array|Get(acopy) _outactors)
      (:Is%20Valid
        (bind _output_get (Variables|Default|SetPlatform (Utilities|Array|Get(acopy) _outactors)))
        (Actor|DestroyActor _output_get)))))

(fn StartingLevelHUD
  (bind _asbp_ball_player_controller (Utilities|Casting|CastToBP_BallPlayerController (Game|GetPlayerController 0)))
  (Default|CallPuttingHUD _asbp_ball_player_controller))